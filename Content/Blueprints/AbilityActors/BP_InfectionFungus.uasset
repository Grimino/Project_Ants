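; Infection fungus ability actor that grows on spawn, disrupts nearby ants and expires after a stat-driven duration.
; A looping timer pulses over the game manager's ant lists, attracting workers, frightening tenders and aggroing soldiers within radius.
; Timelines scale the mesh for growth and shrinking, with a game-over check on fungus death when no infections remain.
; Death, also triggered by depleted HP, returns affected workers and soldiers to their tasks before destroying the actor.
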(event Custom|Event_StartEffectArea
  ;[1 1 1] Start the pulse area effect
  (CallFunction|FunctionAoePulseLogic))

(event Custom|Event_StartGrowth
  ;[1 1 1] Growth animation timeline
  (bind _growthalpha (Timeline|Timeline_FungusGrowth PlayFromStart)
    (:Update
      (Transformation|SetRelativeScale3D (Variables|Default|GetSkeletalMesh) (Math|Vector|MakeVector (Math|Float|Lerp 0.01 0.04 _growthalpha) (Math|Float|Lerp 0.01 0.04 _growthalpha) (Math|Float|Lerp 0.01 0.04 _growthalpha)))
      (Animation|Montage|PlayMontage (Variables|Default|GetSkeletalMesh) "/Game/FO_Folder/FungoAbilita/MushRoomAbility2_Anim_Montage.MushRoomAbility2_Anim_Montage"))))

(event Custom|Event_ReverseGrowth
  ;[1 1 1] Growth animation timeline
  (bind _newtrack_0 (Timeline|Timeline_ReverseGrowth PlayFromStart)
    (:Update
      (Transformation|SetRelativeScale3D (Variables|Default|GetSkeletalMesh) (Math|Vector|MakeVector (Math|Float|Lerp 0.04 0.01 _newtrack_0) (Math|Float|Lerp 0.04 0.01 _newtrack_0) (Math|Float|Lerp 0.04 0.01 _newtrack_0))))
    (:Finished
      (CallFunction|FunctionDeath))))

(event EventBeginPlay
  (|Setthestats)
  (|Setthereferences)
  ;[1 1 1] Set the life span
  (Utilities|Time|SetTimerbyEvent (EventDispatchers|CreateEvent :!event FunctionFungusDeath) (Variables|Static|GetStatic_FungusDuration))
  (|Startgrowthanimation)
  ;[1 1 1] Start the pulse area effect
  (Utilities|Time|SetTimerbyEvent (delegate Custom|Event_StartEffectArea) 1.0 true))

(event EventFunctionFungusDeath
  (Utilities|FlowControl|DoOnce false
    (:Completed
      (if (<= (Variables|/Game/Blueprints/MainCharacter/BP_MainCharacter.BP_MainCharacter_C|GetVariable_InfectionCount (Variables|Default|GetReference_MainCharacter)) 0)
        (CallFunction|EventReverseGrowth)
        (Default|FunctionFungusGameOverCheck (Variables|Default|GetReference_MainCharacter))
        (else
          (CallFunction|EventReverseGrowth))))))

(event EventTick
  (params (DeltaSeconds :type Float%20%28single-precision%29)))

(event EventFunctionInterveneDamage
  (params (InterveneDMG :type Float%20%28double-precision%29))
  ;[1 1 1] Interface functions
  (|Takedamage InterveneDMG))

(fn ConstructionScript)

(fn FunctionAoePulseLogic
  (for _array_element (Variables|/Game/FrameWorks/Managers/BP_GameManager.BP_GameManager_C|GetDynamic_TotalAnts_Worker (Variables|Reference|GetReference_GameManager))
    (if (<= (Transformation|GetDistanceTo _array_element self) (Variables|Static|GetStatic_FungusRadius))
      (Class|IWorkerInterface|FunctionFungusAttraction(Message) _array_element self)
      (Utilities|Array|Add (Variables|Default|GetVariable_WorkerAntsAttracted) _array_element)))
  (for _array_element_2 (Variables|/Game/FrameWorks/Managers/BP_GameManager.BP_GameManager_C|GetDynamic_TotalAnts_Tender (Variables|Reference|GetReference_GameManager))
    (if (<= (Transformation|GetDistanceTo _array_element_2 self) (Variables|Static|GetStatic_FungusRadius))
      (Class|IAntInterface|FunctionAntFear(Message) _array_element_2 (Variables|Static|GetStatic_TenderFearDuration) self)))
  (for _array_element_3 (Variables|/Game/FrameWorks/Managers/BP_GameManager.BP_GameManager_C|GetDynamic_TotalAnts_Soldier (Variables|Reference|GetReference_GameManager))
    (if (<= (Transformation|GetDistanceTo _array_element_3 self) (Variables|Static|GetStatic_FungusRadius))
      (Class|IAntInterface|FunctionFocusChase(Message) _array_element_3 self)
      (Utilities|Array|Add (Variables|Default|GetVariable_SoldierAntsAggro) _array_element_3))))

(fn FunctionDeath
  (for _array_element (Variables|Default|GetVariable_WorkerAntsAttracted)
    (Class|IAntInterface|FunctionReturntoMainTask(Message) _array_element))
  (for _array_element_2 (Variables|Default|GetVariable_SoldierAntsAggro)
    (Class|IAntInterface|FunctionReturntoMainTask(Message) _array_element_2))
  (Actor|DestroyActor))