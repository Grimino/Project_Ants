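; Timed mushroom ability actor that damages and frightens nearby uninfected ants and draws soldier ants to attack it.
; On BeginPlay it scales up via a timeline, takes HP and lifespan from ability stats, and orders soldiers from BP_GameManager within aggro range to chase it.
; An initial sphere-trace pulse, if it hits, starts a looping timer that repeats the pulse through I_AntInterface.
; Incoming damage destroys it at zero HP.
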(event Custom|Event_StartPulse
  (bind _returnvalue (Transformation|GetActorLocation))
  (bind _ds_abilitystats (Variables|Default|GetDS_AbilityStats))
  (bind (_int_ability1charges _int_ability2charges _int_ability3charges _int_ability4charges _float_mycosynthduration _vector_mycosyntharea _float_pheromonesduration _float_pheromonesarea _float_pheromonesfearduration _float_mycosynthsoldierinvestigaterange _float_fungusarearadius _float_funguspulsedamage _float_fungusfearduration) (Utilities|Struct|BreakDS_AbilityStats _ds_abilitystats))
  (bind (_outhits _returnvalue_2) (Class|KismetSystemLibrary|SphereTraceMultibyProfile _returnvalue _returnvalue (.Float_FungusAreaRadius (Utilities|Struct|BreakDS_AbilityStats (Variables|Default|GetDS_AbilityStats))) "None" false 0 "None" true))
  (if _returnvalue_2
    (for _array_element _outhits
      (if (Utilities|DoesObjectImplementInterface (.HitActor (Collision|BreakHitResult _array_element)) "/Game/FrameWorks/Interfaces/I_AntInterface.I_AntInterface_C")
        (bind _isinfected_ (Class|IAntInterface|FunctionInfectionCheck(Message) (.HitActor (Collision|BreakHitResult _array_element))))
        (if (not _isinfected_)
          (Class|IDamageableInterface|FunctionTakeDamage(Message) (.HitActor (Collision|BreakHitResult _array_element)) _float_funguspulsedamage)
          (Class|IAntInterface|FunctionAntFear(Message) (.HitActor (Collision|BreakHitResult _array_element)) _float_fungusfearduration self))))))

(event EventBeginPlay
  (|ScaleMushRoom
    (:NewParam2
      (|Setthefungusstats)
      (|SoldierAggroCheck
        (:Completed
          (|AreaPulseEffect
            (:Completed
              (Utilities|Time|SetTimerbyEvent (delegate Custom|Event_StartPulse) (.Float_FungusPulseFrequency (Utilities|Struct|BreakDS_AbilityStats (Variables|Default|GetDS_AbilityStats))) true))))))))

(event Collision|EventActorBeginOverlap
  (params (OtherActor :type Actor%20Object%20Reference)))

(event EventTick
  (params (DeltaSeconds :type Float%20%28single-precision%29)))

(event EventFunctionTakeDamage
  (params (DamageDealt :type Float%20%28double-precision%29))
  (bind _output_get (Variables|Default|SetStatic_HPValue (- (Variables|Default|GetStatic_HPValue) DamageDealt)))
  (if (<= _output_get 0.0)
    (Actor|DestroyActor)))

(fn ConstructionScript)

(event Custom|MPoint
  (bind _newtrack_0 (Timeline|Timeline Play)
    (:Update
      (Transformation|SetRelativeScale3D (Variables|Default|GetSK_MushRoom) (Math|Vector|MakeVector (Math|Float|Lerp 0.01 0.04 _newtrack_0) (Math|Float|Lerp 0.01 0.04 _newtrack_0) (Math|Float|Lerp 0.01 0.04 _newtrack_0)))
      (Animation|Montage|PlayMontage (Variables|Default|GetSK_MushRoom) "/Game/FO_Folder/FungoAbilita/MushRoomAbility2_Anim_Montage.MushRoomAbility2_Anim_Montage"))))