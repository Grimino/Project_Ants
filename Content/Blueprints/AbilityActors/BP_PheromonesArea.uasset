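; Pheromone ability actor that lives for a configured duration, repeatedly affecting nearby ants.
; A looping half-second timer sphere-traces Pawns, using radius and fear duration from DSAbilityStruct, and messages hit actors through I_AntInterface.
; Infected ants chase a random actor from the externally filled ignore list, while uninfected ants fear this actor.
; The one-shot InitialArea fear pass is temporarily disabled, and the pulse draws debug traces.
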(event Custom|Event_Start%20Pulsing%20Area
  (|PulsingArea))

(event EventBeginPlay
  (Actor|SetLifeSpan (.Float_PheromonesDuration (Utilities|Struct|BreakDS_AbilityStats (Variables|Default|GetDS_AbilityStruct))))
  (Utilities|Time|SetTimerbyEvent (delegate Custom|Event_Start%20Pulsing%20Area) 0.5 true))

(event Collision|EventActorBeginOverlap
  (params (OtherActor :type Actor%20Object%20Reference)))

(event EventTick
  (params (DeltaSeconds :type Float%20%28single-precision%29)))

(fn ConstructionScript)

(fn FunctionSetIgnoreTargets
  (params (Actor%20To%20Ignore :type Actor%20Object%20Reference))
  (Utilities|Array|AddUnique (Variables|Default|GetVariable_ActorsToIgnore) Actor%20To%20Ignore))