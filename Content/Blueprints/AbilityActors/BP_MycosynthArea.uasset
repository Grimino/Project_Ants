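; Mycosynth ability area actor that sends a heal message to infected ants within its radius for the duration of the ability.
; BeginPlay runs a sphere trace and starts a looping timer that re-traces and heals infected ants on every pulse.
; Overlap with AffectArea also heals infected arrivals, skipping those already in the healed-ants list.
; ABSetLifeSpan sets the actor's lifespan from the ability duration.
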(event OnComponentBeginOverlap(AffectArea)
  (params (OverlappedComponent :type Primitive%20Component%20Object%20Reference) (OtherActor :type Actor%20Object%20Reference) (OtherComp :type Primitive%20Component%20Object%20Reference) (OtherBodyIndex :type Integer) (bFromSweep :type Boolean) (SweepResult :type Hit%20Result%20Structure%20%28by%20ref%29))
  (|CollisionTriggerCheck OtherActor OtherActor))

(event Custom|TimedCheck
  (|PeriodicCheck))

(event EventBeginPlay
  (|Initialcheck (delegate Custom|TimedCheck)))

(event EventTick
  (params (DeltaSeconds :type Float%20%28single-precision%29)))

(event EventABSetLifeSpan
  (params (AbilityDuration :type Float%20%28double-precision%29))
  (Actor|SetLifeSpan AbilityDuration))

(fn ConstructionScript)

(fn FunctionCheckHealApplication
  (params (ActorToCheck :type Actor%20Object%20Reference))
  (LocalVariables|SetVariable_ActorAlreadyAdded false)
  (bind _array_element (Utilities|Array|ForEachLoopwithBreak (Variables|Default|GetVariable_HealedAnts) :!label _label)
    (:LoopBody
      (if (== _array_element ActorToCheck)
        (bind _output_get (LocalVariables|SetVariable_ActorAlreadyAdded true))
        (goto _label Break)))
    (:Completed
      (return _output_get))))