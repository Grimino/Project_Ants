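; BP_BaseAbility is an ability targeting actor that can be moved to a drop location and swaps its Target Niagara effect per ability.
; While infection mode is active, Tick sphere-traces for pawns implementing a target-ants interface and shows a valid or invalid effect.
; Other visual setters disable that mode and apply a fixed colored effect.
; A timeline lerps the ability sphere toward the target for a drop animation.
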(event Custom|Event_StartSphereDrop
  (bind _newtrack_0 (Timeline|Timeline_SphereDrop PlayFromStart)
    (:Update
      (|ChangeSphereLocation _newtrack_0))))

(event EventBeginPlay)

(event EventTick
  (params (DeltaSeconds :type Float%20%28single-precision%29))
  (bind _returnvalue (Transformation|GetActorLocation))
  (if (Variables|Default|GetStatic_IsUsingInfection?)
    (bind (_outhits _returnvalue_2) (Collision|MultiSphereTraceForObjects _returnvalue _returnvalue 7e+02 (Utilities|Array|MakeArray "ObjectTypeQuery3") false 0 "None" true "(R=0.000000,G=0.284090,B=1.000000,A=1.000000)"))
    (if _returnvalue_2
      (bind _array_element (Utilities|Array|ForEachLoopwithBreak _outhits :!label _label)
        (:LoopBody
          (if (Utilities|DoesObjectImplementInterface (.HitActor (Collision|BreakHitResult _array_element)) (Variables|Default|GetStatic_AntsToTarget))
            (Variables|Default|SetStatic_IsWorkerAntsFound? true)
            (goto _label Break)
            (else
              (Variables|Default|SetStatic_IsWorkerAntsFound? false))))
        (:Completed
          (if (Variables|Default|GetStatic_IsWorkerAntsFound?)
            (CallFunction|FunctionChangeColor "/Game/FrameWorks/VisualFeedback/Niagaras/NS_TargetAbilityTrue.NS_TargetAbilityTrue")
            (else
              (CallFunction|FunctionChangeColor "/Game/FrameWorks/VisualFeedback/Niagaras/NS_TargetAbilityFalse.NS_TargetAbilityFalse")))))
      (else
        (CallFunction|FunctionChangeColor "/Game/FrameWorks/VisualFeedback/Niagaras/NS_TargetAbilityFalse.NS_TargetAbilityFalse")))))

(fn ConstructionScript)

(fn FunctionSetDropLocation
  (params (NewParam :type Vector))
  (Transformation|SetActorLocation NewParam false false))

(fn FunctionChangeColor
  (params (Color%20To%20Change :type Niagara%20System%20Object%20Reference))
  (Class|NiagaraComponent|SetAsset (Variables|Default|GetTarget) Color%20To%20Change true)
  (return))

(fn FunctionSetAbility1Visual
  (Variables|Default|SetStatic_IsUsingInfection? false)
  (CallFunction|FunctionChangeColor "/Game/FrameWorks/VisualFeedback/AbiliyActor/MycoSintesi/NS_TargetAbilityGreen.NS_TargetAbilityGreen"))

(fn FunctionSetMainInfectionVisual
  (Variables|Default|SetStatic_IsUsingInfection? true))

(fn FunctionSetAbility4Visual
  (Variables|Default|SetStatic_IsUsingInfection? false)
  (CallFunction|FunctionChangeColor "/Game/FrameWorks/VisualFeedback/AbiliyActor/1PointActionTarget/NS_TargetAbilityPurple.NS_TargetAbilityPurple"))

(fn FunctionSetAbility2Visual
  (Variables|Default|SetStatic_IsUsingInfection? false)
  (CallFunction|FunctionChangeColor "/Game/FrameWorks/VisualFeedback/AbiliyActor/1PointActionTarget/NS_TargetAbilityYellow.NS_TargetAbilityYellow"))