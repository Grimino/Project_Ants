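; Ant pawn that walks a loop of waypoints, can be infected, and is destroyed when its health drops below zero.
; Tick uses a resettable DoOnce to set rotation and run the MoveTo macro, which advances the waypoint index after each successful AI move.
; Infection happens once, adding a BPC_Infection component and swapping move speed and material.
; Incoming damage is subtracted from health after a cooldown delay.
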(event EventBeginPlay
  (Variables|Default|SetVariable_ArrayLenght (Utilities|Array|Length (Variables|Default|GetStatic_WayPoints)))
  (Variables|/Script/Engine.FloatingPawnMovement|SetMaxSpeed (Variables|Default|GetFloatingPawnMovement) (Variables|Default|GetStatic_BaseMoveSpeed)))

(event Collision|EventActorBeginOverlap
  (params (OtherActor :type Actor%20Object%20Reference)))

(event EventTick
  (params (DeltaSeconds :type Float%20%28single-precision%29))
  (if (>= (Variables|Default|GetStatic_HealthValue) 0.0)
    (Utilities|FlowControl|DoOnce false :!label _label
      (:Completed
        (Transformation|SetActorRotation (|RotationFinder))
        (|MoveTo
          (:OutputPin
            (if (Variables|Default|GetVariable_IsInfected)
              (goto _label Reset)
              (else
                (goto _label Reset)))))))
    (else
      (Actor|DestroyActor))))

(event EventFunctionInfect
  (Utilities|FlowControl|DoOnce false
    (:Completed
      (Variables|Default|SetVariable_IsInfected true)
      (bind _returnvalue (Game|AddComponentbyClass "/Game/Blueprints/Ants/BPC_Infection.BPC_Infection_C"))
      (Default|FunctionGetAnt _returnvalue self (Variables|Default|GetVariable_IsInfected))
      (Variables|/Script/Engine.FloatingPawnMovement|SetMaxSpeed (Variables|Default|GetFloatingPawnMovement) (Variables|Default|GetStatic_InfectedMoveSpee))
      (Rendering|Material|SetMaterial (Variables|Default|GetSkeletalMesh) 0 "/Engine/MapTemplates/Materials/BasicAsset01.BasicAsset01"))))

(event EventFunctionDealDamage
  (params (DmgAmmount :type Float%20%28double-precision%29))
  (Utilities|FlowControl|Delay (Variables|Default|GetStatic_InfectionDmgCooldown))
  (Variables|Default|SetStatic_HealthValue (- (Variables|Default|GetStatic_HealthValue) DmgAmmount)))

(fn ConstructionScript)