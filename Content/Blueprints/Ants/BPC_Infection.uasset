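; Infection component for ants that spreads infection and damage from an infected ant to nearby ants.
; GetAnt stores the target ant and its infected flag.
; Every Tick runs a debug-drawn multi-sphere trace for Pawns around that ant.
; While the flag is set, hits implementing I_AntInterface receive infect and fixed-damage messages each frame, without delta-time scaling.
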(event EventBeginPlay)

(event EventTick
  (params (DeltaSeconds :type Float%20%28single-precision%29))
  (bind _variable_targetant (Variables|Default|GetVariable_TargetAnt))
  (bind _rootcomponent (Variables|/Script/Engine.Actor|GetRootComponent _variable_targetant))
  (bind _returnvalue (Transformation|GetWorldLocation _rootcomponent))
  (bind _outhits (Collision|MultiSphereTraceForObjects _returnvalue _returnvalue 3e+02 (Utilities|Array|MakeArray "ObjectTypeQuery3") false 0 "ForOneFrame"))
  (for _array_element _outhits
    (if (and (Utilities|DoesObjectImplementInterface (.HitActor (Collision|BreakHitResult _array_element)) "/Game/FrameWorks/Interfaces/I_AntInterface.I_AntInterface_C") (Variables|Default|GetVariable_IsInfected))
      (Class|IAntInterface|FunctionInfect(Message) (.HitActor (Collision|BreakHitResult _array_element)))
      (Class|IAntInterface|FunctionDealDamage(Message) (.HitActor (Collision|BreakHitResult _array_element)) (Variables|Default|GetStatic_InfectionDamage)))))

(fn FunctionGetAnt
  (params (AntToInfect :type Actor%20Object%20Reference) (IsInfected :type Boolean))
  (Variables|Default|SetVariable_TargetAnt AntToInfect)
  (Variables|Default|SetVariable_IsInfected IsInfected))