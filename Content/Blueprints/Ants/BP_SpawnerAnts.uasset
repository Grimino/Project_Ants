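; BP_SpawnerAnts spawns AI-controlled ants at its Box component until the healthy ant population reaches the target held by BP_GameManager.
; It finds the game manager on BeginPlay and compares its target count with the healthy ants array length every Tick.
; A DoOnce gate that resets after a cooldown Delay throttles spawning to one ant at a time.
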(event EventBeginPlay
  (bind _returnvalue (Actor|GetActorOfClass "/Game/FrameWorks/Managers/BP_GameManager.BP_GameManager_C"))
  (Variables|Default|SetReference_GameManager _returnvalue))

(event EventTick
  (params (DeltaSeconds :type Float%20%28single-precision%29))
  (bind _reference_gamemanager (Variables|Default|GetReference_GameManager))
  (if (> (Variables|/Game/FrameWorks/Managers/BP_GameManager.BP_GameManager_C|GetDynamic_TotalAntsToSpawn _reference_gamemanager) (Utilities|Array|Length (Variables|/Game/FrameWorks/Managers/BP_GameManager.BP_GameManager_C|GetDynamic_TotalHealthyAnts _reference_gamemanager)))
    (Utilities|FlowControl|DoOnce false :!label _label
      (:Completed
        (AI|SpawnAIFromClass (Variables|Default|GetDynamic_AntToSpawn) 0 (Transformation|GetWorldLocation (Variables|Default|GetBox)) "0, 0, 0" false 0)
        (Utilities|FlowControl|Delay (Variables|Default|GetStatic_AntSpawnCooldown))
        (goto _label Reset)))))

(fn ConstructionScript)