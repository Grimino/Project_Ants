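; BP_QueenAnt_Parent is the queen ant structure that generates larvae as a resource on a looping timer.
; Init registers the queen with BP_GameManager and sets up drop zones, which are handed out at random; larvae can be taken and counted.
; Hovering shows an outline overlay, and clicking sends health to the game mode's stats panel.
; At zero health it deregisters, alarms all healthy ants and destroys itself.
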(event OnBeginCursorOver(Box)
  (params (TouchedComponent :type Primitive%20Component%20Object%20Reference))
  ;[1 1 1] MouseOver
  (Rendering|Material|SetOverlayMaterial (Variables|Default|GetSkeletal%20Mesh) "/Game/Materials/Outlines/MT_LarvaOutline.MT_LarvaOutline" :!class /Script/Engine.MeshComponent))

(event OnEndCursorOver(Box)
  (params (TouchedComponent :type Primitive%20Component%20Object%20Reference))
  ;[1 1 1] MouseOver
  (Rendering|Material|SetOverlayMaterial (Variables|Default|GetSkeletal%20Mesh) 0 :!class /Script/Engine.MeshComponent))

(event OnClicked(Box)
  (params (TouchedComponent :type Primitive%20Component%20Object%20Reference) (ButtonPressed :type Key%20Structure :default "None"))
  (bind _returnvalue (Game|GetGameMode))
  ;[1 1 1] Click Events
  (Class|IGameModeInterface|GameModeFunctionGetStructureStats(Message) _returnvalue (Variables|Default|GetStatic_HealthValue) 3)
  (Class|IGameModeInterface|GameModeFunctionOpenStatsPanel(Message) _returnvalue)
  (Class|IGameModeInterface|GaneModeFunctionSetClickedObject(Message) _returnvalue self))

(event Custom|Event_LarvaeGeneration
  (Variables|Default|SetStatic_CurrentLarvaeCount (+ (Variables|Default|GetStatic_CurrentLarvaeCount) (Variables|Default|GetStatic_LarvaeGenValue)))
  (Rendering|Components|TextRender|SetText (Variables|Default|GetLarvaeCount) (Utilities|Text|ToText(Integer) (Variables|Default|GetStatic_CurrentLarvaeCount))))

(event Custom|Event_StartGeneration
  (Utilities|Time|SetTimerbyEvent (delegate Custom|Event_LarvaeGeneration) (Variables|Default|GetStatic_LarvaGenCooldown) true))

(event Custom|Event_RefreshUiStats
  (|CollapseGraph))

(event EventBeginPlay
  (Utilities|FlowControl|Delay 0.1)
  (|Init))

(event EventTick
  (params (DeltaSeconds :type Float%20%28single-precision%29)))

(event EventFunctionTakeDamage
  (params (DamageDealt :type Float%20%28double-precision%29))
  (Variables|Default|SetStatic_HealthValue (- (Variables|Default|GetStatic_HealthValue) DamageDealt))
  (if (<= (Variables|Default|GetStatic_HealthValue) 0.0)
    (CallFunction|FunctionDestroyQueen)))

(event EventFunctionTakeResource
  (bind _result (Math|Integer|DecrementInt (Variables|Default|GetStatic_CurrentLarvaeCount))
    (:%20%20
      (Variables|Default|SetStatic_CurrentLarvaeCount (Math|Integer|Clamp(Integer) _result 0 999)))))

(fn ConstructionScript)

(fn FunctionDestroyQueen
  (bind _reference_gm (Variables|Default|GetReference_GM))
  (Class|IGMInterface|FunctionRemoveStructure(Message) (Variables|Default|GetReference_GM) (Variables|Default|GetStatic_StructureID) 0 0 self)
  (for _array_element (Variables|/Game/FrameWorks/Managers/BP_GameManager.BP_GameManager_C|GetDynamic_TotalHealthyAnts _reference_gm)
    (Class|IAntInterface|FunctionAlarmedAlert(Message) _array_element))
  (Variables|/Game/FrameWorks/Managers/BP_GameManager.BP_GameManager_C|SetDynamic_IsInAlarmedState _reference_gm true)
  (Actor|DestroyActor))

(fn FunctionGiveAntDropZones
  (return (.OutItem (Utilities|Array|Random (Variables|Default|GetVariable_DropZones)))))

(fn FunctionCheckRemainingFood
  (return (Variables|Default|GetStatic_CurrentLarvaeCount)))