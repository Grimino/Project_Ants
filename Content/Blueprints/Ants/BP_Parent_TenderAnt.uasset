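; Parent Blueprint for tender ants, which haul food from the food supply to the ant spawner until infected.
; An enum state machine on Tick runs DoOnce-gated AI moves for working, waiting, fleeing and alarmed wandering.
; Interface calls switch states, and depleted health triggers infection.
; Infected ants alert nearby ants, then chase and bite GameManager-assigned targets while decaying toward death, which triggers a game-over check.
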(event Custom|Event_DecayingHealth
  ;[1 0 0.03419] Custom events
  (Math|Float|DecrementFloat (Variables|Static|GetStatic_InfectedHealth)))

(event Custom|Event_StartDecayHealth
  ;[1 0 0.03419] Custom events
  (Utilities|Time|SetTimerbyEvent (delegate Custom|Event_DecayingHealth) 1.0 true))

(event EventBeginPlay
  ;[1 0 0.8717] Begin play init
  (|Init))

(event EventFunctionProximityAlert
  (params (NearbyAnt :type Actor%20Object%20Reference))
  ;[0 1 0.09148] Interface functions
  (if (not (Variables|Variable|GetVariable_IsInfected))
    (Class|NavMovementComponent|StopActiveMovement (Variables|Character|GetCharacterMovement))
    (Variables|Reference|SetReference_NearbyInfectedAnt NearbyAnt)
    (CallFunction|FunctionDropFood)
    (Variables|Default|SetEM_TenderStateMachine "NewEnumerator1")))

(event EventTick
  (params (DeltaSeconds :type Float%20%28single-precision%29))
  ;[0 0.03257 1] State machine
  (if (<= (Variables|Static|GetStatic_InfectedHealth) 0.0)
    (Variables|Default|SetEM_TenderStateMachine "NewEnumerator7"))
  (switch Utilities|FlowControl|Switch|SwitchonEM_TenderAntState (Variables|Default|GetEM_TenderStateMachine)
    (:NewEnumerator8
      (|MainTask_Behaviour_2))
    (:NewEnumerator9
      (|SecondaryTask_Behaviour))
    (:NewEnumerator1
      (|Proximity_Behaviour_2))
    (:NewEnumerator2
      (|Alarmed_Behaviour_2))
    (:NewEnumerator3
      (Utilities|FlowControl|DoOnce false
        (:Completed
          (|Infected_Behaviour_2))))
    (:NewEnumerator4
      (|Chase_Behaviour_2))
    (:NewEnumerator6
      (|Attack_Behaviour_2))
    (:NewEnumerator7
      (CallFunction|FunctionDeath))))

(event EventFunctionInfect
  ;[0 1 0.09148] Interface functions
  (if (not (Variables|Variable|GetVariable_IsInfected))
    (Variables|Default|SetEM_TenderStateMachine "NewEnumerator3")))

(event EventFunctionGetNewStructure
  (params (StructureID :type Integer))
  (bind _reference_gmreference (Variables|Variable|GetReference_GmReference))
  (if (not (Variables|Variable|GetVariable_IsInfected))
    (Development|PrintText "Changing structure!")
    (switch int StructureID
      (:1
        (bind _food_supply (Default|FunctionGiveFoodSupply _reference_gmreference))
        (Variables|Reference|SetReference_FoodSupply _food_supply))
      (:2
        (bind _antspawner (Default|FunctionGiveAntSpawner _reference_gmreference))
        (Variables|Reference|SetReference_AntSpawner _antspawner)))
    (Class|NavMovementComponent|StopActiveMovement (Variables|Character|GetCharacterMovement))
    (CallFunction|FunctionReturntoMainTask)))

(event EventFunctionReturntoMainTask
  ;[0 1 0.09148] Interface functions
  (if (not (Variables|Variable|GetVariable_IsInfected))
    (Class|NavMovementComponent|StopActiveMovement (Variables|Character|GetCharacterMovement))
    (Variables|Default|SetEM_TenderStateMachine "NewEnumerator8")))

(event EventFunctionAlarmedAlert
  ;[0 1 0.09148] Interface functions
  (if (not (Variables|Variable|GetVariable_IsInfected))
    (Class|NavMovementComponent|StopActiveMovement (Variables|Character|GetCharacterMovement))
    (Variables|Default|SetEM_TenderStateMachine "NewEnumerator2")))

(event EventFunctionInterveneDamage
  (params (InterveneDamage :type Float%20%28double-precision%29))
  ;[0 1 0.09148] Interface functions
  (Variables|Static|SetStatic_InfectedHealth (- (Variables|Static|GetStatic_InfectedHealth) InterveneDamage)))

(event EventFunctionTakeDamage
  (params (DamageDealt :type Float%20%28double-precision%29))
  ;[0 1 0.09148] Interface functions
  (|DealDamage DamageDealt))

(fn ConstructionScript)

(fn FunctionInfectedBite
  (bind _reference_attacktarget (Variables|Reference|GetReference_AttackTarget))
  (Utilities|IsValid (Variables|Reference|GetReference_AttackTarget)
    (:Is%20Valid
      (Class|IDamageableInterface|FunctionTakeDamage(Message) _reference_attacktarget (Variables|Static|GetStatic_BiteDamage))
      (bind _healthremaining (Class|IAntInterface|FunctionInfectionCheck(Message) _reference_attacktarget))
      (if (>= _healthremaining 0.0)
        (Class|IAntInterface|FunctionProximityAlert(Message) (Variables|Reference|GetReference_AttackTarget) self)
        (else
          (Class|IAntInterface|FunctionInfect(Message) (Variables|Reference|GetReference_AttackTarget)))))
    (:Is%20Not%20Valid
      (Class|NavMovementComponent|StopActiveMovement (Variables|Character|GetCharacterMovement))
      (Variables|Default|SetEM_TenderStateMachine "NewEnumerator4"))))

(fn FunctionDropFood
  (Variables|Variable|SetVariable_IsHoldingFood? false)
  (Development|SetHiddeninGame (Variables|Default|GetHoldedFood) true false))

(fn FunctionDeath
  (bind _reference_gmreference (Variables|Variable|GetReference_GmReference))
  (Default|FunctionRemoveInfectedAnt _reference_gmreference self)
  (Default|GameOverCheck _reference_gmreference)
  (Actor|DestroyActor))

(fn FunctionsGotoSecondaryTask
  (Class|NavMovementComponent|StopActiveMovement (Variables|Character|GetCharacterMovement))
  (Variables|Default|SetEM_TenderStateMachine "NewEnumerator9"))

(fn FunctionActivateFood
  (Variables|Variable|SetVariable_IsHoldingFood? true)
  (Development|SetHiddeninGame (Variables|Default|GetHoldedFood) false false))

(fn FunctionInfectionCheck
  (return (Variables|Variable|GetVariable_IsInfected) (Variables|Static|GetStatic_HealthValue) (Variables|Static|GetStatic_InfectedHealth)))