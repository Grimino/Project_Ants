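; Parent ant pawn that patrols waypoints, can take delayed damage or be infected, and registers with BP_GameManager.
; A Tick-driven enum state machine uses DoOnce gates to loop AI moves: Idle cycles waypoints, Infected wanders to random reachable points.
; Infection adds BPC_Infection and changes speed and material, but the state switches and notifies the manager only upon reaching the next waypoint.
; Only Idle checks health to destroy the ant.
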(event EventBeginPlay
  (Variables|Default|SetEM_StateMachine "NewEnumerator0")
  (Variables|Variable|SetVariable_ArrayLenght (Utilities|Array|Length (Variables|Static|GetStatic_WayPoints)))
  (Variables|/Script/Engine.FloatingPawnMovement|SetMaxSpeed (Variables|Default|GetFloatingPawnMovement) (Variables|Static|GetStatic_BaseMoveSpeed))
  (bind _returnvalue (Actor|GetActorOfClass "/Game/FrameWorks/Managers/BP_GameManager.BP_GameManager_C"))
  (Default|FunctionGetAnt _returnvalue self))

(event Collision|EventActorBeginOverlap
  (params (OtherActor :type Actor%20Object%20Reference)))

(event EventTick
  (params (DeltaSeconds :type Float%20%28single-precision%29))
  (switch Utilities|FlowControl|Switch|SwitchonEM_AntState (Variables|Default|GetEM_StateMachine)
    (:NewEnumerator0
      (|Idle_Behaviour))
    (:NewEnumerator3
      (|Infected_Behaviour))))

(event EventFunctionInfect
  (Utilities|FlowControl|DoOnce false
    (:Completed
      (|InfectionLogic))))

(event EventFunctionDealDamage
  (params (DmgAmmount :type Float%20%28double-precision%29))
  (Utilities|FlowControl|Delay (Variables|Static|GetStatic_InfectionDmgCooldown))
  (Variables|Static|SetStatic_HealthValue (- (Variables|Static|GetStatic_HealthValue) DmgAmmount)))

(fn ConstructionScript)