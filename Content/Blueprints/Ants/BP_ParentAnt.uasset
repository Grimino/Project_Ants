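; Parent ant Blueprint for a colony infection simulation, driven by an enum state machine on Tick and registered with BP_GameManager.
; Idle ants ferry food between sources and supplies given by the manager.
; At zero health they become infected, lose health each second until destroyed, and after a delay chase and bite the nearest healthy ant.
; Proximity alerts hide carried food and switch state, but the flee logic is disconnected.
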(event Custom|Event_DecayingHealth
  (Math|Float|DecrementFloat (Variables|Default|GetStatic_InfectedHealth)))

(event Custom|Event_StartDecayHealth
  (Utilities|Time|SetTimerbyEvent (delegate Custom|Event_DecayingHealth) 1.0 true))

(event EventBeginPlay
  (Variables|/Script/Engine.CharacterMovementComponent|SetMaxWalkSpeed (Variables|Character|GetCharacterMovement) (Variables|Static|GetStatic_BaseMoveSpeed))
  (Variables|Default|SetEM_StateMachine "NewEnumerator0")
  (bind _returnvalue (Actor|GetActorOfClass "/Game/FrameWorks/Managers/BP_GameManager.BP_GameManager_C"))
  (Variables|Variable|SetReference_GmReference _returnvalue)
  (Default|FunctionGetAnt (Variables|Variable|GetReference_GmReference) self))

(event EventFunctionProximityAlert
  (params (NearbyAnt :type Actor%20Object%20Reference))
  (Variables|Default|SetReference_NearbyInfectedAnt NearbyAnt)
  (if (not (Variables|Variable|GetVariable_IsInfected))
    (Development|PrintString "help!" true true "(R=1.000000,G=0.949367,B=0.000000,A=1.000000)" 0.18)
    (Variables|Default|SetEM_StateMachine "NewEnumerator1")
    (Variables|Variable|SetVariable_IsHoldingFood? false)
    (Rendering|SetVisibility (Variables|Default|GetHoldedFood) false false)))

(event EventTick
  (params (DeltaSeconds :type Float%20%28single-precision%29))
  (if (<= (Variables|Default|GetStatic_InfectedHealth) 0.0)
    (Variables|Default|SetEM_StateMachine "NewEnumerator7"))
  (switch Utilities|FlowControl|Switch|SwitchonEM_AntState (Variables|Default|GetEM_StateMachine)
    (:NewEnumerator0
      (|Idle_Behaviour_2))
    (:NewEnumerator1
      (|Proximity_Behaviour))
    (:NewEnumerator3
      (Utilities|FlowControl|DoOnce false
        (:Completed
          (|Infected_Behaviour))))
    (:NewEnumerator4
      (|Chase_Behaviour))
    (:NewEnumerator6
      (|Attack_Behaviour))
    (:NewEnumerator7
      (Default|FunctionRemoveInfectedAnt (Variables|Variable|GetReference_GmReference) self)
      (Actor|DestroyActor))))

(event EventFunctionInfect
  (Variables|Default|SetEM_StateMachine "NewEnumerator3"))

(event EventFunctionDealDamage
  (params (DmgAmmount :type Float%20%28double-precision%29))
  (Variables|Static|SetStatic_HealthValue (- (Variables|Static|GetStatic_HealthValue) DmgAmmount))
  (if (<= (Variables|Static|GetStatic_HealthValue) 0.0)
    (CallFunction|FunctionInfect)))

(fn ConstructionScript)

(fn FunctionInfectedBite
  (Class|IAntInterface|FunctionDealDamage(Message) (Variables|Default|GetReference_NearestAnt) (Variables|Default|GetStatic_BiteDamage)))