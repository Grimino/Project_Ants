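; Wandering ant pawn that registers with BP_GameManager and can be infected.
; Tick uses a DoOnce to rotate and AI-move toward helper-generated random points (apparently away from the player), re-arming only on success, and destroys the ant once health drops below zero.
; Infection happens once, adding BPC_Infection and changing speed and material; damage lands after a cooldown delay.
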(event EventBeginPlay
  (Variables|/Script/Engine.FloatingPawnMovement|SetMaxSpeed (Variables|Default|GetFloatingPawnMovement) (Variables|StaticValues|GetStatic_BaseMoveSpeed))
  (bind _returnvalue (Actor|GetActorOfClass "/Game/FrameWorks/Managers/BP_GameManager.BP_GameManager_C"))
  (Default|FunctionGetAnt _returnvalue self))

(event Collision|EventActorBeginOverlap
  (params (OtherActor :type Actor%20Object%20Reference)))

(event EventTick
  (params (DeltaSeconds :type Float%20%28single-precision%29))
  (bind _randomlocation (|RandomPoint_2))
  (if (>= (Variables|StaticValues|GetStatic_HealthValue) 0.0)
    (Utilities|FlowControl|DoOnce false :!label _label
      (:Completed
        (Transformation|SetActorRotation (|GetRandomPointRotation_2 _randomlocation))
        (AI|AIMoveTo self _randomlocation 0 1e+01 false
          (:OnSuccess
            (if (Variables|Variablevalues|GetVariable_IsInfected)
              (goto _label Reset)
              (else
                (goto _label Reset)))))))
    (else
      (Actor|DestroyActor))))

(event EventFunctionInfect
  (Utilities|FlowControl|DoOnce false
    (:Completed
      (Variables|Variablevalues|SetVariable_IsInfected true)
      (bind _returnvalue (Game|AddComponentbyClass "/Game/Blueprints/Ants/BPC_Infection.BPC_Infection_C"))
      (Default|FunctionGetAnt _returnvalue self (Variables|Variablevalues|GetVariable_IsInfected))
      (Variables|/Script/Engine.FloatingPawnMovement|SetMaxSpeed (Variables|Default|GetFloatingPawnMovement) (Variables|StaticValues|GetStatic_InfectedMoveSpee))
      (Rendering|Material|SetMaterial (Variables|Default|GetSkeletalMesh) 0 "/Engine/MapTemplates/Materials/BasicAsset01.BasicAsset01"))))

(event EventFunctionDealDamage
  (params (DmgAmmount :type Float%20%28double-precision%29))
  (Utilities|FlowControl|Delay (Variables|StaticValues|GetStatic_InfectionDmgCooldown))
  (Variables|StaticValues|SetStatic_HealthValue (- (Variables|StaticValues|GetStatic_HealthValue) DmgAmmount)))

(fn ConstructionScript)