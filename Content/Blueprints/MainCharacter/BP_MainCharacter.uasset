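; Player-controlled camera character that roams the level, follows ants and infects them through cursor clicks.
; Enhanced Input drives movement, camera-relative mouse drag, key or mouse yaw rotation, and stepped spring-arm zoom with interpolation.
; Cursor traces find I_AntInterface pawns: Interact spends a limited infection count, while starting mouse rotation over an ant locks on to it.
; Tick snaps the actor to the followed ant until move or drag input releases it.
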(event Custom|ResetCamera
  (Variables|Variable|SetVariable_IsCamFollowing false)
  (Utilities|FlowControl|DoOnce false) ; enters at Reset
)

(event Input|EnhancedActionEvents|EnhancedInputActionIA_Move
  (params (ActionValue :type Vector%202D%20Structure) (ElapsedSeconds :type Float%20%28double-precision%29) (TriggeredSeconds :type Float%20%28double-precision%29) (InputAction :type Input%20Action%20Object%20Reference :default "/Game/FrameWorks/InputMappings/IA_Move.IA_Move"))
  ;[0 1 0.2031] Movement Inputs
  (:Triggered
    (|CollapseGraph (.x ActionValue) (.y ActionValue)))
  (:Started
    (CallFunction|ResetCamera)))

(event Input|EnhancedActionEvents|EnhancedInputActionIA_CameraDrag
  (params (ActionValue :type Boolean) (ElapsedSeconds :type Float%20%28double-precision%29) (TriggeredSeconds :type Float%20%28double-precision%29) (InputAction :type Input%20Action%20Object%20Reference :default "/Game/FrameWorks/InputMappings/IA_CameraDrag.IA_CameraDrag"))
  ;[0.849 0 0.03117] Camera Drag
  (:Triggered
    (|Drag))
  (:Started
    (bind _returnvalue (Class|WidgetLayoutLibrary|GetMousePositiononViewport))
    (Variables|Variable|SetVariable_PreviousClickLocation _returnvalue)
    (CallFunction|ResetCamera)))

(event Input|EnhancedActionEvents|EnhancedInputActionIA_KeyRotation
  (params (ActionValue :type Float%20%28double-precision%29) (ElapsedSeconds :type Float%20%28double-precision%29) (TriggeredSeconds :type Float%20%28double-precision%29) (InputAction :type Input%20Action%20Object%20Reference :default "/Game/FrameWorks/InputMappings/IA_KeyRotation.IA_KeyRotation"))
  ;[0 0.272 1] Camera Rotation
  (:Triggered
    (|Q/ERotation ActionValue)))

(event Input|EnhancedActionEvents|EnhancedInputActionIA_Interact
  (params (ActionValue :type Boolean) (ElapsedSeconds :type Float%20%28double-precision%29) (TriggeredSeconds :type Float%20%28double-precision%29) (InputAction :type Input%20Action%20Object%20Reference :default "/Game/FrameWorks/InputMappings/IA_Interact.IA_Interact"))
  ;[1 0 0.9911] Interact
  (:Started
    (|Interact)))

(event Input|EnhancedActionEvents|EnhancedInputActionIA_Zoom
  (params (ActionValue :type Boolean) (ElapsedSeconds :type Float%20%28double-precision%29) (TriggeredSeconds :type Float%20%28double-precision%29) (InputAction :type Input%20Action%20Object%20Reference :default "/Game/FrameWorks/InputMappings/IA_Zoom.IA_Zoom"))
  ;[1 0.7216 0] Camera Zoom
  (:Triggered
    (|Zoom)))

(event Input|EnhancedActionEvents|EnhancedInputActionIA_MouseRotation
  (params (ActionValue :type Boolean) (ElapsedSeconds :type Float%20%28double-precision%29) (TriggeredSeconds :type Float%20%28double-precision%29) (InputAction :type Input%20Action%20Object%20Reference :default "/Game/FrameWorks/InputMappings/IA_MouseRotation.IA_MouseRotation"))
  ;[0 0.272 1] Camera Rotation
  (:Triggered
    (|MouseRotation))
  (:Started
    (|CameraFollow)))

(event EventBeginPlay
  (Input|AddMappingContext)
  (Variables|/Script/Engine.PlayerController|SetbShowMouseCursor (Game|GetPlayerController 0) true))

(event EventTick
  (params (DeltaSeconds :type Float%20%28single-precision%29))
  (bind _reference_anttofollow (Variables|Reference|GetReference_AntToFollow))
  (if (Variables|Variable|GetVariable_IsCamFollowing)
    (Utilities|IsValid _reference_anttofollow
      (:Is%20Valid
        (Transformation|SetActorLocation (Transformation|GetActorLocation _reference_anttofollow) false false))
      (:Is%20Not%20Valid
        (Utilities|FlowControl|DoOnce false :!label _label
          (:Completed
            (Transformation|SetActorLocation (Transformation|GetActorLocation) false false)))))
    (else
      (goto _label))))

(fn ConstructionScript)