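; Ant spawner landmark that turns deposited food into new ants and shows its stored food count on a text render.
; On Init it registers with BP_GameManager, which holds the ant class and population counts.
; Each tick, enough food is spent to raise the manager's spawn target, subject to a cap.
; While healthy ants fall short of that target, it spawns AI ants at its box after a short delay.
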(event EventBeginPlay
  (|Init))

(event EventFunctionDepositFood
  (params (FoodDropValue :type Integer))
  (Variables|Default|SetStatic_FoodCount (+ FoodDropValue (Variables|Default|GetStatic_FoodCount))))

(event EventTick
  (params (DeltaSeconds :type Float%20%28single-precision%29))
  (bind _reference_gamemanager (Variables|Default|GetReference_GameManager))
  (bind _reference_gamemanager_2 (Variables|Default|GetReference_GameManager))
  (Rendering|Components|TextRender|SetText (Variables|Default|GetTextRender) (Utilities|Text|ToText(Integer) (Variables|Default|GetStatic_FoodCount)))
  (if (>= (Variables|Default|GetStatic_FoodCount) (Variables|Default|GetStatic_FoodToSpawnAnt))
    (Variables|Default|SetStatic_FoodCount (Math|Integer|Clamp(Integer) (- (Variables|Default|GetStatic_FoodCount) (Variables|Default|GetStatic_FoodToSpawnAnt)) 0 999))
    (if (<= (Variables|/Game/FrameWorks/Managers/BP_GameManager.BP_GameManager_C|GetDynamic_TotalAntsToSpawn _reference_gamemanager_2) (Variables|Default|GetStatic_MaxAntSpawnable))
      (Variables|/Game/FrameWorks/Managers/BP_GameManager.BP_GameManager_C|SetDynamic_TotalAntsToSpawn _reference_gamemanager_2 (+ (Variables|/Game/FrameWorks/Managers/BP_GameManager.BP_GameManager_C|GetDynamic_TotalAntsToSpawn _reference_gamemanager_2) (Variables|/Game/FrameWorks/Managers/BP_GameManager.BP_GameManager_C|GetStatic_AntstoAddInScene _reference_gamemanager_2)))
      (if (> (Variables|/Game/FrameWorks/Managers/BP_GameManager.BP_GameManager_C|GetDynamic_TotalAntsToSpawn _reference_gamemanager) (Utilities|Array|Length (Variables|/Game/FrameWorks/Managers/BP_GameManager.BP_GameManager_C|GetDynamic_TotalHealthyAnts _reference_gamemanager))) :!label _label
        (Utilities|FlowControl|Delay 0.2)
        (AI|SpawnAIFromClass (Variables|/Game/FrameWorks/Managers/BP_GameManager.BP_GameManager_C|GetDynamic_AntToSpawn (Variables|Default|GetReference_GameManager)) 0 (Transformation|GetWorldLocation (Variables|Default|GetBox)) "0, 0, 0" false 0)))
    (else
      (goto _label))))

(fn ConstructionScript)

(fn FunctionGetFood
  (params (FoodRequested :type Integer))
  (return 0))