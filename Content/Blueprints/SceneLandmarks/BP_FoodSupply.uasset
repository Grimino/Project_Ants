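; BP_FoodSupply is a food stockpile landmark that stores a food count and shows it on a text render updated every tick.
; On BeginPlay it finds BP_GameManager and passes itself to it.
; A deposit event adds food without a cap, while FunctionGetFood subtracts the request with clamping, then returns the lesser of the request and the already reduced count.
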(event EventBeginPlay
  (bind _returnvalue (Actor|GetActorOfClass "/Game/FrameWorks/Managers/BP_GameManager.BP_GameManager_C"))
  (bind _output_get (Variables|Default|SetReference_GameManager _returnvalue))
  (Class|IGMInterface|FunctionGetFoodSupply(Message) _output_get self))

(event EventFunctionDepositFood
  (params (FoodDropValue :type Integer))
  (Variables|Default|SetStatic_FoodCount (+ FoodDropValue (Variables|Default|GetStatic_FoodCount))))

(event EventTick
  (params (DeltaSeconds :type Float%20%28single-precision%29))
  (Rendering|Components|TextRender|SetText (Variables|Default|GetTextRender) (Utilities|Text|ToText(Integer) (Variables|Default|GetStatic_FoodCount))))

(fn ConstructionScript)

(fn FunctionGetFood
  (params (FoodRequested :type Integer))
  (bind _output_get (Variables|Default|SetVariable_FoodRequested FoodRequested))
  (Variables|Default|SetStatic_FoodCount (Math|Integer|Clamp(Integer) (- (Variables|Default|GetStatic_FoodCount) _output_get) 0 999))
  (if (>= FoodRequested (Variables|Default|GetStatic_FoodCount))
    (Variables|Default|SetVariable_FoodGiven (Variables|Default|GetStatic_FoodCount))
    (else
      (Variables|Default|SetVariable_FoodGiven (Variables|Default|GetVariable_FoodRequested))))
  (return (Variables|Default|GetVariable_FoodGiven)))