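; Interactable scene object that toggles between a solid physical mesh and a glass phantom of the same configurable mesh.
; The interface call FunctionActivate flips state: activation moves the physical mesh onto the phantom and hides it, while deactivation reveals the phantom and moves the physical mesh to WayPoint before hiding it.
; Timelines lerp from the current location, with DoOnce and Delay providing per-direction cooldowns.
; Cursor hover applies outline overlay materials.
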(event OnBeginCursorOver(PhantomObjectMesh)
  (params (TouchedComponent :type Primitive%20Component%20Object%20Reference))
  (Rendering|Material|SetOverlayMaterial (Variables|Default|GetPhantomObjectMesh) "/Game/Materials/Outlines/MT_IoBOutLine.MT_IoBOutLine" :!class /Script/Engine.MeshComponent))

(event OnEndCursorOver(PhantomObjectMesh)
  (params (TouchedComponent :type Primitive%20Component%20Object%20Reference))
  (Rendering|Material|SetOverlayMaterial (Variables|Default|GetPhantomObjectMesh) 0 :!class /Script/Engine.MeshComponent))

(event OnBeginCursorOver(PhysicalObjectMesh)
  (params (TouchedComponent :type Primitive%20Component%20Object%20Reference))
  (Rendering|Material|SetOverlayMaterial (Variables|Default|GetPhysicalObjectMesh) "/Game/Materials/Outlines/MT_ObjectOutline.MT_ObjectOutline" :!class /Script/Engine.MeshComponent))

(event OnEndCursorOver(PhysicalObjectMesh)
  (params (TouchedComponent :type Primitive%20Component%20Object%20Reference))
  (Rendering|Material|SetOverlayMaterial (Variables|Default|GetPhysicalObjectMesh) 0 :!class /Script/Engine.MeshComponent))

(event Custom|Event_Activate
  ;[1 1 1] Activate the object
  (Utilities|FlowControl|DoOnce false :!label _label
    (:Completed
      (Development|SetHiddeninGame (Variables|Default|GetPhysicalObjectMesh) false false)
      (|Activate_Timelinelogics
        (:Finished
          (goto _label Reset))))))

(event Custom|Event_Deactivate
  ;[1 1 1] Deactivate the Object
  (Utilities|FlowControl|DoOnce false :!label _label
    (:Completed
      (Development|SetHiddeninGame (Variables|Default|GetPhantomObjectMesh) false false)
      (|Activate_Timelinelogics_2
        (:Finished
          (goto _label Reset))))))

(event EventBeginPlay
  ;[1 1 1] Init
  (|SetStaticMeshesandMaterials)
  (if (not (Variables|Default|GetStatic_StartActivated?))
    (CallFunction|EventDeactivate)))

(event EventTick
  (params (DeltaSeconds :type Float%20%28single-precision%29)))

(event EventFunctionActivate
  ;[1 1 1] Interface Functions
  (if (Variables|Default|GetVariable_IsActivated)
    (CallFunction|EventDeactivate)
    (else
      (CallFunction|EventActivate))))

(fn ConstructionScript)