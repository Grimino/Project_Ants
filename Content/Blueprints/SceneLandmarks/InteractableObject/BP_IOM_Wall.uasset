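; Clickable wall that toggles between its original transform and a target, moving to a waypoint actor, rotating to an arrow's orientation, or both.
; BeginPlay caches both rotations and the start location; clicks choose out or back from a moved flag.
; Timeline macros lerp from the cube's current transform, with DoOnce blocking re-triggers until a cooldown delay ends.
; Yellow material marks activity, red follows cooldown, and hover adds an outline overlay.
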(event OnBeginCursorOver(Cube)
  (params (TouchedComponent :type Primitive%20Component%20Object%20Reference))
  ;[1 1 1] MouseOver
  (Rendering|Material|SetOverlayMaterial (Variables|Default|GetCube) "/Game/Materials/Outlines/MT_IOMoutline.MT_IOMoutline" :!class /Script/Engine.MeshComponent))

(event OnEndCursorOver(Cube)
  (params (TouchedComponent :type Primitive%20Component%20Object%20Reference))
  ;[1 1 1] MouseOver
  (Rendering|Material|SetOverlayMaterial (Variables|Default|GetCube) 0 :!class /Script/Engine.MeshComponent))

(event OnClicked(Cube)
  (params (TouchedComponent :type Primitive%20Component%20Object%20Reference) (ButtonPressed :type Key%20Structure :default "None"))
  ;[1 1 1] Interface functions
  (if (Variables|Variable|GetVariable_HasMoved?)
    (CallFunction|EventMoveBack)
    (else
      (CallFunction|EventMoveOut))))

(event Custom|Event_MoveOut
  ;[1 1 1] Move and/or rotate Object to Waypoint
  (Utilities|FlowControl|Sequence
    (:then_0
      (if (Variables|Variable|GetVariable_ChangePosition?)
        (|MovementA)))
    (:then_1
      (if (Variables|Variable|GetVariable_ChangeRotation?)
        (|RotationA :!label _label
          (:OutputPin
            (goto _label Reset)))))))

(event Custom|Event_MoveBack
  ;[1 1 1] Move and/or Object to Original Position
  (Utilities|FlowControl|Sequence
    (:then_0
      (if (Variables|Variable|GetVariable_ChangePosition?)
        (|MovementB)))
    (:then_1
      (if (Variables|Variable|GetVariable_ChangeRotation?)
        (|RotationB)))))

(event EventBeginPlay
  ;[1 1 1] Init
  (Variables|Variable|SetVariable_OriginalPosition (Transformation|GetWorldLocation (Variables|Default|GetCube)))
  (Variables|Variable|SetVariable_OriginalRotation (Transformation|GetWorldRotation (Variables|Default|GetCube)))
  (Variables|Variable|SetVariable_ArrowRotation (Transformation|GetWorldRotation (Variables|Default|GetRotationView))))

(event EventTick
  (params (DeltaSeconds :type Float%20%28single-precision%29)))

(fn ConstructionScript)