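; BP_IOB_Wall is an interactable wall object that switches between a passable glass state and a solid red state.
; Each FunctionActivate call runs a FlipFlop: the first swaps the Cube to glass material and disables its collision, the next swaps it to red and restores query and physics collision.
; Both branches print a debug message naming the new state.
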(event EventBeginPlay)

(event EventTick
  (params (DeltaSeconds :type Float%20%28single-precision%29)))

(event EventFunctionActivate
  (Utilities|FlowControl|FlipFlop
    (:A
      (Development|PrintText "Deactivated")
      (Rendering|Material|SetMaterial (Variables|Default|GetCube) 0 "/Game/MSPresets/M_MS_Glass_Material/MI_MS_Glass_Material_Inst.MI_MS_Glass_Material_Inst")
      (Collision|SetCollisionEnabled (Variables|Default|GetCube) "NoCollision"))
    (:B
      (Development|PrintText "Activated")
      (Rendering|Material|SetMaterial (Variables|Default|GetCube) 0 "/Game/Materials/MT_Red.MT_Red")
      (Collision|SetCollisionEnabled (Variables|Default|GetCube) "QueryAndPhysics"))))

(fn ConstructionScript)