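; BP_FoodSupply is a food stockpile actor that tracks a food count and displays it on a text render.
; On BeginPlay it finds BP_GameManager and passes itself to it through FunctionGetFoodSupplyMessage.
; FunctionDepositFood adds StaticFoodValue to StaticFoodCount.
; The text is refreshed from that count every Tick rather than on each deposit.
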(event EventBeginPlay
  (bind _returnvalue (Actor|GetActorOfClass "/Game/FrameWorks/Managers/BP_GameManager.BP_GameManager_C"))
  (Class|IGMInterface|FunctionGetFoodSupply(Message) _returnvalue self))

(event EventFunctionDepositFood
  (Variables|Default|SetStatic_FoodCount (+ (Variables|Default|GetStatic_FoodValue) (Variables|Default|GetStatic_FoodCount))))

(event EventTick
  (params (DeltaSeconds :type Float%20%28single-precision%29))
  (Rendering|Components|TextRender|SetText (Variables|Default|GetTextRender) (Utilities|Text|ToText(Integer) (Variables|Default|GetStatic_FoodCount))))

(fn ConstructionScript)