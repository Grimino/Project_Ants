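; BP_SCUI is an actor for a 3D suitcase UI that films its prop meshes (books, bag, cap and other objects) with a SceneCaptureComponent2D.
; On BeginPlay it plays a montage on the cap's skeletal mesh, then registers each prop as a show-only component so the capture is limited to them.
; A debug "Hello" print follows, and Tick, overlap and the construction script are empty.
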(event EventBeginPlay
  (bind _78_book_01 (Variables|Default|Get78_book_01))
  (bind _78_book_08 (Variables|Default|Get78_Book_08))
  (bind _78_object004 (Variables|Default|Get78_Object004))
  (bind _78_cylinder038 (Variables|Default|Get78_Cylinder038))
  (bind _78_cap001 (Variables|Default|Get78_cap001))
  (bind _78_book_011 (Variables|Default|Get78_Book_011))
  (bind _78_book_09 (Variables|Default|Get78_Book_09))
  (bind _78_bag001 (Variables|Default|Get78_bag001))
  (bind _78_book_03 (Variables|Default|Get78_Book_03))
  (bind _78_line005 (Variables|Default|Get78_Line005))
  (bind _78_book_05 (Variables|Default|Get78_Book_05))
  (bind _78_cylinder019 (Variables|Default|Get78_Cylinder019))
  (bind _array (Utilities|Array|MakeArray _78_book_01 _78_book_08 _78_object004 _78_cylinder038 _78_cap001 _78_book_011 _78_book_09 _78_bag001 _78_book_03 _78_line005 _78_book_05 _78_cylinder019))
  (Utilities|Array|Add _array 0)
  (Animation|Montage|PlayMontage (Variables|Default|Get78_cap001) "/Game/FO_Folder/UI3D_MM/HUD_Test/ASSET_UI3D/old-pitchman-suitcase/source/78_cap001_Anim_Montage.78_cap001_Anim_Montage"
    (:then
      (for _array_element _array
        (Rendering|SceneCapture|ShowOnlyComponent (Variables|Default|GetSceneCaptureComponent2D) _array_element))
      (Development|PrintString "Hello"))))

(event Collision|EventActorBeginOverlap
  (params (OtherActor :type Actor%20Object%20Reference)))

(event EventTick
  (params (DeltaSeconds :type Float%20%28single-precision%29)))

(fn ConstructionScript)