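; BP_Menu3D is a world-space 3D menu actor that moves the player's view between linked menu actors.
; On BeginPlay it binds to its Menu3DWidget's transition event and disables its own collision.
; A transition index selects an entry in LinkedMenus, swaps collision from this menu to the target, and eases the player's view target to it with SetViewTargetWithBlend.
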(event Custom|TransictionTo
  (params (NewMenu :type BP%20Menu%203D%20Object%20Reference))
  (Collision|SetActorEnableCollision false)
  (Collision|SetActorEnableCollision NewMenu true)
  (Game|Player|SetViewTargetwithBlend (Game|GetPlayerController 0) NewMenu 2.0 "VTBlend_EaseInOut" 2.0 false))

(event Custom|OnTransitionBetweenMenus
  (params (MenuIndex :type Integer))
  (if (Utilities|Array|IsValidIndex (Variables|Default|GetLinkedMenus) MenuIndex)
    (CallFunction|Transictionto (Utilities|Array|Get(acopy) (Variables|Default|GetLinkedMenus) MenuIndex))))

(event EventBeginPlay
  (bind _asmenu_3dwidget (Utilities|Casting|CastToMenu3DWidget (UserInterface|GetUserWidgetObject (Variables|Default|GetWidget))))
  (EventDispatchers|BindEventtoTransitiontoLinkedMenu _asmenu_3dwidget (delegate Custom|OnTransitionBetweenMenus))
  (Collision|SetActorEnableCollision false))

(fn ConstructionScript)