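; Skills manager actor that runs the player's four charge-based ant abilities and the main infection fungus placement.
; A gated Tick traces from the mouse to move a BP_BaseAbility targeting visual while targeting is on.
; Abilities spend charges loaded from a data struct, refresh UI through the GameMode, and spawn effects at that location.
; Mycosynth and pheromones also send nearby soldier or infected ants from the GameManager's lists to investigate.
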(event Custom|Event_TurnOnArea
  (params (AbilitySwitch :type EM_AbilityTypes%20Enum :default "NewEnumerator0") (MainInfection :type Boolean))
  (|SpawnVisualeffectsarea AbilitySwitch MainInfection)
  (Utilities|FlowControl|Gate true) ; enters at Open
)

(event Custom|Event_TurnOffArea
  (|Despawnvisualsandcleararray)
  (Utilities|FlowControl|Gate true) ; enters at Close
)

(event Custom|Event_MainInfectionAbility
  (CallFunction|FunctionSpawnInfectionFungus (Variables|Variable|GetVariable_MouseLocation)))

(event Custom|Event_Ability4
  (Math|Integer|DecrementInt (Variables|Static|GetStatic_Ability4Charges)
    (:%20%20
      (|UpdateUICharges_4)
      (CallFunction|ABBerserkArea))))

(event Custom|Event_Abilty1
  (Math|Integer|DecrementInt (Variables|Static|GetStatic_Ability1Charges)
    (:%20%20
      (CallFunction|FunctionCallSphereDrop)
      (CallFunction|ABMycosynthHeal)
      (CallFunction|FunctionSoldierPriorityCall)
      (|UpdateUIcharges))))

(event Custom|Event_Ability2
  (Math|Integer|DecrementInt (Variables|Static|GetStatic_Ability2Charges)
    (:%20%20
      (CallFunction|FunctionInfectedPheromonesInvestigate)
      (|UpdateUICharges2))))

(event Custom|Event_Ability3
  (Math|Integer|DecrementInt (Variables|Static|GetStatic_Ability3Charges)
    (:%20%20
      (|UpdateUICharges3)
      (CallFunction|ABWaterDrop))))

(event EventBeginPlay
  (Utilities|FlowControl|Delay 0.2)
  (bind _returnvalue (Actor|GetActorOfClass "/Game/Blueprints/MainCharacter/BP_MainCharacter.BP_MainCharacter_C"))
  (Variables|Reference|SetReference_MainCharacter _returnvalue)
  (bind _returnvalue_2 (Actor|GetActorOfClass "/Game/FrameWorks/Managers/BP_GameManager.BP_GameManager_C"))
  (Variables|Reference|SetReference_GameManager _returnvalue_2)
  (|Setthestatsofthestruct))

(event EventTick
  (params (DeltaSeconds :type Float%20%28single-precision%29))
  (Utilities|FlowControl|Gate true
    (:Exit
      (CallFunction|FunctionFindTargetedArea (Variables|Static|GetStatic_TargetAreaRadius)))))

(fn ConstructionScript)

(fn FunctionGetTargetedAntsinArea
  (bind _variable_mouselocation (Variables|Variable|GetVariable_MouseLocation))
  (bind (_outhits _returnvalue) (Class|KismetSystemLibrary|SphereTraceMultibyProfile _variable_mouselocation _variable_mouselocation (Variables|Static|GetStatic_TargetAreaRadius) "Pawn" false 0 "None" true))
  (if _returnvalue
    (for _array_element _outhits
      (if (Utilities|DoesObjectImplementInterface (.HitActor (Collision|BreakHitResult _array_element)) "/Game/FrameWorks/Interfaces/I_AntInterface.I_AntInterface_C")
        (bind _isinfected_ (Class|IAntInterface|FunctionInfectionCheck(Message) (.HitActor (Collision|BreakHitResult _array_element))))
        (if _isinfected_
          (Utilities|Array|AddUnique (Variables|Variable|GetVariable_AntsToTarget) (.HitActor (Collision|BreakHitResult _array_element))))))
    (return (Variables|Variable|GetVariable_AntsToTarget))))

(fn FunctionFindTargetedArea
  (params (AreaRadius :type Float%20%28double-precision%29))
  (bind _returnvalue (Game|GetPlayerController 0))
  (bind (_worldlocation _worlddirection) (Game|Player|ConvertMouseLocationToWorldSpace _returnvalue))
  (bind (_outhit _returnvalue_2) (Collision|LineTraceByChannel _worldlocation (+ _worldlocation (* _worlddirection 1e+04)) "TraceTypeQuery2" false 0 "None" true "(R=1.000000,G=0.000000,B=0.000000,A=1.000000)" "(R=0.000000,G=1.000000,B=0.000000,A=1.000000)" 0.2))
  (if _returnvalue_2
    (bind _output_get (Variables|Variable|SetVariable_MouseLocation (.Location (Collision|BreakHitResult _outhit))))
    (Transformation|SetActorLocation (Variables|Default|GetReference_AbilityVisual) _output_get false false)
    (return)))

(fn ABMycosynthHeal
  (bind _returnvalue (Game|SpawnActorfromClass "/Game/Blueprints/AbilityActors/BP_MycosynthArea.BP_MycosynthArea_C" (Math|Transform|MakeTransform (Variables|Variable|GetVariable_MouseLocation) "0, 0, 0" (Variables|Static|GetStatic_MycosynthArea)) "Undefined" "MultiplyWithRoot" 0 0))
  (Class|IAbilityInterface|ABSetLifeSpan(Message) _returnvalue (Variables|Static|GetStatic_MycosynthDuration))
  (Variables|Default|SetVariable_InvestigateLocation (Transformation|GetActorLocation _returnvalue)))

(fn FunctionCallSphereDrop
  (Default|EventStartSphereDrop (Variables|Default|GetReference_AbilityVisual)))

(fn FunctionSoldierPriorityCall
  (for _array_element (Variables|/Game/FrameWorks/Managers/BP_GameManager.BP_GameManager_C|GetDynamic_TotalAnts_Soldier (Variables|Reference|GetReference_GameManager))
    (if (<= (Transformation|GetDistanceTo _array_element (Variables|Default|GetReference_AbilityVisual)) (.Float_MycosynthSoldierInvestigateRange (Utilities|Struct|BreakDS_AbilityStats (Variables|Reference|GetReference_AbilityDataStruct))))
      (Class|IAntInterface|FunctionSoldiersInvestigate(Message) _array_element (Variables|Default|GetVariable_InvestigateLocation)))))

(fn FunctionSpawnInfectionFungus
  (params (Location :type Vector))
  (Game|SpawnActorfromClass "/Game/Blueprints/AbilityActors/BP_InfectionFungus.BP_InfectionFungus_C" (Math|Transform|MakeTransform Location "0, 0, 0" "1.000000,1.000000,1.000000") "Undefined" "MultiplyWithRoot" 0 0))

(fn FunctionInfectedPheromonesInvestigate
  (bind (_spawn_location _pheromones) (Default|FunctionSpawnPheromones (Variables|Default|GetReference_AbilityVisual)))
  (Variables|Default|SetVariable_InvestigateLocation _spawn_location)
  (for _array_element (Variables|/Game/FrameWorks/Managers/BP_GameManager.BP_GameManager_C|GetDynamic_TotalInfectedAnts (Variables|Reference|GetReference_GameManager))
    (if (<= (Transformation|GetDistanceTo _array_element _pheromones) (.Float_PheromonesArea (Utilities|Struct|BreakDS_AbilityStats (Variables|Reference|GetReference_AbilityDataStruct))))
      (Class|IAntInterface|ABPheromonesInvestigate(Message) _array_element (Variables|Variable|GetVariable_MouseLocation)))))

(fn ABWaterDrop
  (bind _returnvalue (Game|SpawnActorfromClass "/Game/Blueprints/AbilityActors/BP_WaterDrop.BP_WaterDrop_C" (Math|Transform|MakeTransform (Variables|Variable|GetVariable_MouseLocation) "0, 0, 0" "1.000000,1.000000,1.000000") "Undefined" "MultiplyWithRoot" 0 0))
  (Default|FunctionSetWaterLifeSpan _returnvalue (.Float_WaterDropDuration (Utilities|Struct|BreakDS_AbilityStats (Variables|Reference|GetReference_AbilityDataStruct)))))

(fn ABBerserkArea
  (bind _returnvalue (Game|SpawnActorfromClass "/Game/Blueprints/AbilityActors/BP_BerserkArea.BP_BerserkArea_C" (Math|Transform|MakeTransform (Variables|Variable|GetVariable_MouseLocation) "0, 0, 0" "1.000000,1.000000,1.000000") "Undefined" "MultiplyWithRoot" 0 0))
  (Default|FunctionSetBerserkAreaDuration _returnvalue (.Float_BerserkAreaDuration (Utilities|Struct|BreakDS_AbilityStats (Variables|Reference|GetReference_AbilityDataStruct)))))