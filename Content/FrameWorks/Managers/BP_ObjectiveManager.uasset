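; BP_ObjectiveManager tracks ant-game objectives (food pile, spawners, queen, healthy ants) and handles the win/lose condition.
; Check events tell BP_UIManager to create objective widgets, flagging queen death and cleared spawners.
; When BP_GameManager lists no infected ants, a resettable timer leads to GameOver, which shows a win or lose message.
; The queen-and-spawner check deciding that result leaves both flags unconnected, and FunctionGetAttackTarget is an empty stub.
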(event Custom|ResetGameOverTimer
  ;[0 1 0.1601] WIN/LOSE CON
  (Utilities|Time|ClearandInvalidateTimerbyHandle (Variables|References|GetReference_GameOverTimer))
  (Variables|Variables|SetVariable_IsChecking? false)
  (Development|PrintText "CLEAR"))

(event Custom|GameOverCheck
  ;[0 1 0.1601] WIN/LOSE CON
  (if (<= (Utilities|Array|Length (Variables|/Game/FrameWorks/Managers/BP_GameManager.BP_GameManager_C|GetDynamic_TotalInfectedAnts (Variables|References|GetReference_GameManager))) 0)
    (bind _returnvalue (Utilities|Time|SetTimerbyEvent (delegate Custom|GameOver) (Variables|Default|GetStatic_GameOverTime)))
    (Variables|References|SetReference_GameOverTimer _returnvalue)
    (Variables|Variables|SetVariable_IsChecking? true)))

(event Custom|GameOver
  ;[0 1 0.1601] WIN/LOSE CON
  (if (|CheckifQueenisdeadandnoSpawnerisleft)
    (Class|IUIInterface|FunctionWin(Message) (Variables|References|GetReference_UIManager))
    (else
      (Class|IUIInterface|FunctionLose(Message) (Variables|References|GetReference_UIManager)))))

(event Custom|QueenCheck
  (Default|CreateObjectivesWidgets (Variables|References|GetReference_UIManager) 2)
  (Variables|Variables|SetVariable_IsQueenDead? true))

(event Custom|SpawnersCheck
  (Default|CreateObjectivesWidgets (Variables|References|GetReference_UIManager) 1)
  (Variables|Variables|SetVariable_NoSpawnersLeft? true))

(event Custom|FoodPileCheck
  (Default|CreateObjectivesWidgets (Variables|References|GetReference_UIManager)))

(event Custom|HealthyAntsCheck
  (if (Utilities|Array|IsEmpty (Variables|/Game/FrameWorks/Managers/BP_GameManager.BP_GameManager_C|GetDynamic_TotalHealthyAnts (Variables|References|GetReference_GameManager)))
    (Default|CreateObjectivesWidgets (Variables|References|GetReference_UIManager) 3)))

(event EventBeginPlay
  (bind _returnvalue (Actor|GetActorOfClass "/Game/FrameWorks/Managers/BP_GameManager.BP_GameManager_C"))
  (Variables|References|SetReference_GameManager _returnvalue)
  (bind _returnvalue_2 (Actor|GetActorOfClass "/Game/FrameWorks/Managers/BP_UIManager.BP_UIManager_C"))
  (Variables|References|SetReference_UIManager _returnvalue_2))

(event EventTick
  (params (DeltaSeconds :type Float%20%28single-precision%29)))

(fn ConstructionScript)

(fn FunctionGetAttackTarget
  (params (AntID :type Integer) (AntActor :type Actor%20Object%20Reference))
  (return 0))