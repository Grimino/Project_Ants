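; UI manager actor for an ant infection game that creates the loading screen, in-game HUD, pause menu and game-over screen.
; Events and functions push objective banners, ant and structure stats, ability charges, infection count and time-button graphics into those widgets.
; It also controls game speed (stop, normal, double, triple), inversely scaling the main character's time dilation and rotation speed.
; Objective banner durations are adjusted for faster speeds, and completed objectives are tallied for game over.
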(event Custom|TimeTripleGraphic
  ;[1 0 0.8328] Graphics
  ;;[1 1 1] Time Control
  (|TimeResetandTimeTripleGraphic))

(event Custom|TimeStopGraphic
  ;[1 0 0.8328] Graphics
  ;;[1 1 1] Time Control
  (|TimeResetandTimeStopGraphic))

(event Custom|DeactivateAbilityGlow
  ;[1 0 0.8328] Graphics
  (Default|DeactivateAbilityGlow (Variables|/Game/FrameWorks/Widgets/WBP_InGameUI.WBP_InGameUI_C|GetWBP_TavolaAbilita (Variables|Refernces|GetReference_InGameUI))))

(event Custom|TimeNormalGraphic
  ;[1 0 0.8328] Graphics
  ;;[1 1 1] Time Control
  (|TimeResetandTimeNormalGraphic))

(event Custom|Event_ToggleLoadingScreen
  ;[1 1 1] Loading screen toggle
  (Widget|RemovefromParent (Variables|Default|GetWBP_LoadingScreen))
  (bind _output_get (Variables|Variables|SetVariable_CurrentGlobalTimeDilation 1.0))
  (Utilities|Time|SetGlobalTimeDilation _output_get)
  (bind _returnvalue (UserInterface|CreateWidget "/Game/FrameWorks/Widgets/WBP_InGameUI.WBP_InGameUI_C"))
  (bind _output_get_2 (Variables|Refernces|SetReference_InGameUI _returnvalue))
  (UserInterface|Viewport|AddtoViewport _output_get_2 0))

(event Custom|TimeDoubleGraphic
  ;[1 0 0.8328] Graphics
  ;;[1 1 1] Time Control
  (|TimeResetandTimeDoubleGraphic))

(event Custom|PauseGame
  ;[0 0.01802 1] Pause
  (if (not (Variables|Variables|GetVariable_IsPauseActive))
    (Variables|Variables|SetVariable_IsPauseActive true)
    (bind _returnvalue (UserInterface|CreateWidget "/Game/FrameWorks/Widgets/WBP_PauseMenuComplete.WBP_PauseMenuComplete_C"))
    (bind _output_get (Variables|Refernces|SetReference_PauseMenu _returnvalue))
    (UserInterface|Viewport|AddtoViewport _output_get 0)
    (Input|SetInputModeUIOnly (Game|GetPlayerController 0) _output_get "DoNotLock" false)
    (CallFunction|FunctionTimeStop)
    (else
      (Widget|RemovefromParent (Variables|Refernces|GetReference_PauseMenu))
      (Input|SetInputModeGameandUI (Game|GetPlayerController 0) (Variables|Refernces|GetReference_InGameUI) "DoNotLock" false false)
      (CallFunction|FunctionTimeReset)
      (CallFunction|PauseGraphic)
      (Variables|Variables|SetVariable_IsPauseActive false))))

(event Custom|PauseGraphic
  ;[1 0 0.8328] Graphics
  (Default|ChangeGraphic (Variables|/Game/FrameWorks/Widgets/WBP_InGameUI.WBP_InGameUI_C|GetWBP_PauseButton (Variables|Refernces|GetReference_InGameUI)) true))

(event Custom|InfectionCountGraphic
  ;[1 0 0.8328] Graphics
  (|SetsInfectionCountText))

(event Custom|CreateGameoverScreen
  (params (AllObjectivesComplete :type Boolean))
  (bind _reference_gameoverwidget (Variables|Refernces|GetReference_GameOverWidget))
  ;[1 0.5846 0] OBJECTIVES
  (Default|SetGameOverScreen _reference_gameoverwidget (Utilities|Text|ToText(Integer) (Variables|Variables|GetVariable_CompletedObjectives)) (Utilities|Text|ToText(Integer) (Variables|Static|GetStatic_TotalObjectives)) AllObjectivesComplete)
  (Widget|RemovefromParent (Variables|Refernces|GetReference_InGameUI))
  (Variables|/Script/UMG.Widget|SetVisibility _reference_gameoverwidget "SelfHitTestInvisible")
  (Game|SetGamePaused true))

(event Custom|BannerTimeDilation
  (params (Selection :type Integer))
  ;[1 0.5846 0] OBJECTIVES
  (|Bannerdurationfix Selection))

(event Custom|CreateObjectivesWidgets
  (params (Selection :type Integer))
  ;[1 0.5846 0] OBJECTIVES
  (switch int Selection
    (:0
      (|FoodPileObjective))
    (:1
      (|SpawnersObjective))
    (:2
      (|QueenObjective))
    (:3
      (|HealthyAntsObjective))
    (:4
      (|SingleInfectionObjective))))

(event Custom|StatsPanelGraphic
  (params (GoesUp? :type Boolean))
  ;[1 0 0.8328] Graphics
  (Default|StatsAnimation (Variables|/Game/FrameWorks/Widgets/WBP_InGameUI.WBP_InGameUI_C|GetWBP_SatsAnt (Variables|Refernces|GetReference_InGameUI)) GoesUp?))

(event Custom|AbilitiesGraphic
  (params (AbilityID :type Integer))
  ;[1 0 0.8328] Graphics
  (|ControlsAbilitiesInfoandButtons AbilityID))

(event EventBeginPlay
  (if (Variables|Static|GetStatic_ShowLoadScreen)
    (|LoadingScreen)
    (else
      (|LoadUIifnoloadingscreen)))
  (bind _returnvalue (Actor|GetActorOfClass "/Game/Blueprints/MainCharacter/BP_MainCharacter.BP_MainCharacter_C"))
  (Variables|Refernces|SetReference_MainCharacter _returnvalue)
  (bind _returnvalue_2 (Actor|GetActorOfClass "/Game/FrameWorks/Managers/BP_GameManager.BP_GameManager_C"))
  (Variables|Refernces|SetReference_GameManager _returnvalue_2)
  (bind _returnvalue_3 (UserInterface|CreateWidget "/Game/FrameWorks/Widgets/WBP_GameOver.WBP_GameOver_C"))
  (bind _output_get (Variables|Refernces|SetReference_GameOverWidget _returnvalue_3))
  (UserInterface|Viewport|AddtoViewport _output_get 0)
  (Variables|/Script/UMG.Widget|SetVisibility _output_get "Hidden"))

(event Collision|EventActorBeginOverlap
  (params (OtherActor :type Actor%20Object%20Reference)))

(event EventTick
  (params (DeltaSeconds :type Float%20%28single-precision%29)))

(event EventFunctionDoubleTime
  ;[0 0.904 1] Time Control
  (CallFunction|FunctionTimeDouble))

(event EventFunctionTripleTime
  ;[0 0.904 1] Time Control
  (CallFunction|FunctionTimeTriple))

(event EventFunctionStopTime
  ;[0 0.904 1] Time Control
  (CallFunction|FunctionTimeStop))

(event EventFunctionResetTime
  ;[0 0.904 1] Time Control
  (CallFunction|FunctionTimeReset))

(fn ConstructionScript)

(fn FunctionTimeDouble
  (bind _reference_maincharacter (Variables|Refernces|GetReference_MainCharacter))
  (bind _output_get (Variables|Variables|SetVariable_CurrentGlobalTimeDilation 2.0))
  (Utilities|Time|SetGlobalTimeDilation _output_get)
  (bind _output_get_2 (Variables|/Script/Engine.Actor|SetCustomTimeDilation _reference_maincharacter 0.5))
  (Variables|Variables|SetVariable_CurrentTimeDilation _output_get_2)
  (Variables|/Game/Blueprints/MainCharacter/BP_MainCharacter.BP_MainCharacter_C|SetVariable_CurrentKeyRotationSpeed _reference_maincharacter (* (Variables|/Game/Blueprints/MainCharacter/BP_MainCharacter.BP_MainCharacter_C|GetStatic_KeyRotationSpeed _reference_maincharacter) 0.5))
  (Variables|/Game/Blueprints/MainCharacter/BP_MainCharacter.BP_MainCharacter_C|SetVariable_CurrentMouseRotationSpeed _reference_maincharacter (* (Variables|/Game/Blueprints/MainCharacter/BP_MainCharacter.BP_MainCharacter_C|GetStatic_MouseRotationSpeed _reference_maincharacter) 0.5))
  (Variables|Variables|SetVariable_IsTimeActive true)
  (CallFunction|BannerTimeDilation 1))

(fn FunctionTimeTriple
  (bind _reference_maincharacter (Variables|Refernces|GetReference_MainCharacter))
  (bind _output_get (Variables|Variables|SetVariable_CurrentTimeDilation 3.0))
  (Utilities|Time|SetGlobalTimeDilation _output_get)
  (bind _output_get_2 (Variables|/Script/Engine.Actor|SetCustomTimeDilation _reference_maincharacter 0.333333))
  (Variables|Variables|SetVariable_CurrentTimeDilation _output_get_2)
  (Variables|/Game/Blueprints/MainCharacter/BP_MainCharacter.BP_MainCharacter_C|SetVariable_CurrentKeyRotationSpeed _reference_maincharacter (* (Variables|/Game/Blueprints/MainCharacter/BP_MainCharacter.BP_MainCharacter_C|GetStatic_KeyRotationSpeed _reference_maincharacter) 0.333333))
  (Variables|/Game/Blueprints/MainCharacter/BP_MainCharacter.BP_MainCharacter_C|SetVariable_CurrentMouseRotationSpeed _reference_maincharacter (* (Variables|/Game/Blueprints/MainCharacter/BP_MainCharacter.BP_MainCharacter_C|GetStatic_MouseRotationSpeed _reference_maincharacter) 0.333333))
  (Variables|Variables|SetVariable_IsTimeActive true)
  (CallFunction|BannerTimeDilation 2))

(fn FunctionTimeStop
  (bind _reference_maincharacter (Variables|Refernces|GetReference_MainCharacter))
  (if (Variables|Variables|GetVariable_IsPauseActive)
    (Utilities|Time|SetGlobalTimeDilation 1e-05)
    (else
      (bind _output_get (Variables|Variables|SetVariable_CurrentGlobalTimeDilation 1e-05))
      (Utilities|Time|SetGlobalTimeDilation _output_get)
      (bind _output_get_2 (Variables|/Script/Engine.Actor|SetCustomTimeDilation _reference_maincharacter 1e+04))
      (Variables|Variables|SetVariable_CurrentTimeDilation _output_get_2)
      (Variables|/Game/Blueprints/MainCharacter/BP_MainCharacter.BP_MainCharacter_C|SetVariable_CurrentKeyRotationSpeed _reference_maincharacter (* (Variables|/Game/Blueprints/MainCharacter/BP_MainCharacter.BP_MainCharacter_C|GetStatic_KeyRotationSpeed _reference_maincharacter) 1e+04))
      (Variables|/Game/Blueprints/MainCharacter/BP_MainCharacter.BP_MainCharacter_C|SetVariable_CurrentMouseRotationSpeed _reference_maincharacter (* (Variables|/Game/Blueprints/MainCharacter/BP_MainCharacter.BP_MainCharacter_C|GetStatic_MouseRotationSpeed _reference_maincharacter) 1e+04))
      (Variables|Variables|SetVariable_IsTimeActive false))))

(fn FunctionTimeReset
  (bind _reference_maincharacter (Variables|Refernces|GetReference_MainCharacter))
  (bind _reference_maincharacter_2 (Variables|Refernces|GetReference_MainCharacter))
  (if (Variables|Variables|GetVariable_IsPauseActive)
    (Utilities|Time|SetGlobalTimeDilation (Variables|Variables|GetVariable_CurrentGlobalTimeDilation))
    (bind _output_get (Variables|/Script/Engine.Actor|SetCustomTimeDilation _reference_maincharacter (Variables|Variables|GetVariable_CurrentTimeDilation)))
    (Variables|Variables|SetVariable_CurrentTimeDilation _output_get)
    (Variables|/Game/Blueprints/MainCharacter/BP_MainCharacter.BP_MainCharacter_C|SetVariable_CurrentKeyRotationSpeed _reference_maincharacter (Variables|/Game/Blueprints/MainCharacter/BP_MainCharacter.BP_MainCharacter_C|GetStatic_KeyRotationSpeed _reference_maincharacter))
    (Variables|/Game/Blueprints/MainCharacter/BP_MainCharacter.BP_MainCharacter_C|SetVariable_CurrentMouseRotationSpeed _reference_maincharacter (Variables|/Game/Blueprints/MainCharacter/BP_MainCharacter.BP_MainCharacter_C|GetStatic_MouseRotationSpeed _reference_maincharacter))
    (else
      (bind _output_get_2 (Variables|Variables|SetVariable_CurrentGlobalTimeDilation 1.0))
      (Utilities|Time|SetGlobalTimeDilation _output_get_2)
      (bind _output_get_3 (Variables|/Script/Engine.Actor|SetCustomTimeDilation _reference_maincharacter_2 1.0))
      (Variables|Variables|SetVariable_CurrentTimeDilation _output_get_3)
      (Variables|/Game/Blueprints/MainCharacter/BP_MainCharacter.BP_MainCharacter_C|SetVariable_CurrentKeyRotationSpeed _reference_maincharacter_2 (Variables|/Game/Blueprints/MainCharacter/BP_MainCharacter.BP_MainCharacter_C|GetStatic_KeyRotationSpeed _reference_maincharacter_2))
      (Variables|/Game/Blueprints/MainCharacter/BP_MainCharacter.BP_MainCharacter_C|SetVariable_CurrentMouseRotationSpeed _reference_maincharacter_2 (Variables|/Game/Blueprints/MainCharacter/BP_MainCharacter.BP_MainCharacter_C|GetStatic_MouseRotationSpeed _reference_maincharacter_2))
      (Variables|Variables|SetVariable_IsTimeActive true)))
  (CallFunction|BannerTimeDilation))

(fn FunctionGetAntStats
  (params (Helath :type Float%20%28double-precision%29) (Damage :type Float%20%28double-precision%29) (Speed :type Float%20%28double-precision%29) (AntID :type Integer) (IsInfected? :type Boolean))
  (bind _reference_ingameui (Variables|Refernces|GetReference_InGameUI))
  (bind _wbp_satsant (Variables|/Game/FrameWorks/Widgets/WBP_InGameUI.WBP_InGameUI_C|GetWBP_SatsAnt _reference_ingameui))
  (bind _wbp_satsant_2 (Variables|/Game/FrameWorks/Widgets/WBP_InGameUI.WBP_InGameUI_C|GetWBP_SatsAnt _reference_ingameui))
  (bind _antpotrait (Variables|/Game/FrameWorks/Widgets/WBP_ParametriFormiche/WBP_SatsAnt.WBP_SatsAnt_C|GetAntPotrait _wbp_satsant_2))
  (Widget|SetVisibility (Variables|Variables|GetVariable_ActivePotrait) "Hidden")
  (Widget|SetVisibility (Variables|/Game/FrameWorks/Widgets/WBP_ParametriFormiche/WBP_SatsAnt.WBP_SatsAnt_C|GetSpeedSection _wbp_satsant) "Visible")
  (Variables|Variables|SetVariable_ActivePotrait (Variables|/Game/FrameWorks/Widgets/WBP_ParametriFormiche/WBP_SatsAnt.WBP_SatsAnt_C|GetAntPotrait _wbp_satsant))
  (Variables|/Game/FrameWorks/Widgets/WBP_ParametriFormiche/WBP_SatsAnt.WBP_SatsAnt_C|SetHealthText _wbp_satsant_2 (Utilities|Text|ToText(Float) Helath "HalfToEven"))
  (Variables|/Game/FrameWorks/Widgets/WBP_ParametriFormiche/WBP_SatsAnt.WBP_SatsAnt_C|SetDamageText _wbp_satsant_2 (Utilities|Text|ToText(Float) Damage "HalfToEven"))
  (Variables|/Game/FrameWorks/Widgets/WBP_ParametriFormiche/WBP_SatsAnt.WBP_SatsAnt_C|SetSpeedText _wbp_satsant_2 (Utilities|Text|ToText(Float) Speed "HalfToEven"))
  (switch int AntID
    (:0
      (|SetsWorkerPotraitandText _wbp_satsant_2 _antpotrait))
    (:1
      (|SetsTenderPotraitandText _wbp_satsant_2 _antpotrait))
    (:2
      (|SetsSoldierPotraitandText _antpotrait _wbp_satsant_2))
    (:3
      (|SetsGuardianPotraitandText _antpotrait _wbp_satsant_2))))

(fn FunctionRefreshAbilityCharges
  (params (Ability%20ID :type Integer) (Ability%201 :type Integer) (Ability%202 :type Integer) (Ability%203 :type Integer) (Ability%204 :type Integer))
  (switch int Ability%20ID
    (:0
      (|CollapseGraph Ability%201))
    (:1
      (|CollapseGraph_0 Ability%202))
    (:2
      (|CollapseGraph_1 Ability%203))
    (:3
      (|CollapseGraph_2 Ability%204))))

(fn FunctionGetStructureStats
  (params (Health :type Float%20%28double-precision%29) (StructureID :type Integer))
  (bind _reference_ingameui (Variables|Refernces|GetReference_InGameUI))
  (bind _wbp_satsant (Variables|/Game/FrameWorks/Widgets/WBP_InGameUI.WBP_InGameUI_C|GetWBP_SatsAnt _reference_ingameui))
  (Variables|/Game/FrameWorks/Widgets/WBP_ParametriFormiche/WBP_SatsAnt.WBP_SatsAnt_C|SetHealthText _wbp_satsant (Utilities|Text|ToText(Float) Health "HalfToEven"))
  (Widget|SetVisibility (Variables|/Game/FrameWorks/Widgets/WBP_ParametriFormiche/WBP_SatsAnt.WBP_SatsAnt_C|GetSpeedSection _wbp_satsant) "Hidden")
  (switch int StructureID
    (:0
      (|FoodSource _wbp_satsant))
    (:1
      (|FoodPile _wbp_satsant))
    (:2
      (|LarvaePile _wbp_satsant))
    (:3
      (|QueenAnt _wbp_satsant))))