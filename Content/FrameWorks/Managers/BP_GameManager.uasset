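; Central manager for an ant-colony infection game, tracking healthy, infected and role-specific ants, plus food sources, supplies and spawners.
; Registration functions fill these lists, and getters return random food locations or spawners.
; Each registered ant advances an enum cycle choosing the next spawn: three workers, two tenders, one soldier.
; Tick prints debug counts and alarms healthy ants once when outnumbered; GameOverTimer schedules game over when infection runs out.
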(event Custom|GameOver
  ;[1 0 0] Game Over
  (Class|IUIInterface|FunctionGameOver(Message) (Variables|Default|GetReference_UIManager)))

(event Custom|GameOverTimer
  ;[1 0 0] Game Over
  (if (and (<= (Variables|/Game/Blueprints/MainCharacter/BP_MainCharacter.BP_MainCharacter_C|GetStatic_InfectionCount (Variables|Default|GetReference_MainCharacter)) 0) (<= (Utilities|Array|Length (Variables|Default|GetDynamic_TotalInfectedAnts)) 0))
    (bind _returnvalue (Utilities|Time|SetTimerbyEvent (delegate Custom|GameOver) (Variables|Default|GetStatic_GameOverTime)))
    (Variables|Default|SetReference_GameOverTimer _returnvalue)))

(event EventBeginPlay
  (Utilities|FlowControl|Delay 0.2)
  (Variables|Default|SetReference_EMSpawnLogic "NewEnumerator0")
  (Variables|Default|SetDynamic_AntToSpawn (Variables|Default|GetReference_AntWorker))
  (bind _returnvalue (Actor|GetActorOfClass "/Game/Blueprints/MainCharacter/BP_MainCharacter.BP_MainCharacter_C"))
  (Variables|Default|SetReference_MainCharacter _returnvalue)
  (bind _returnvalue_2 (Actor|GetActorOfClass "/Game/FrameWorks/Managers/BP_UIManager.BP_UIManager_C"))
  (Variables|Default|SetReference_UIManager _returnvalue_2))

(event Collision|EventActorBeginOverlap
  (params (OtherActor :type Actor%20Object%20Reference)))

(event EventFunctionGetWorker
  (params (WorkerAnt :type Actor%20Object%20Reference))
  (Utilities|Array|Add (Variables|Default|GetDynamic_TotalAnts_Worker) WorkerAnt))

(event EventTick
  (params (DeltaSeconds :type Float%20%28single-precision%29))
  (Development|PrintText (Utilities|Text|ToText(Integer) (Utilities|Array|Length (Variables|Default|GetDynamic_TotalHealthyAnts))) true true "(R=0.000000,G=0.660000,B=1.000000,A=1.000000)" 0.008)
  (Development|PrintString (Utilities|String|ToString(Integer) (Utilities|Array|Length (Variables|Default|GetDynamic_TotalInfectedAnts))) true true "(R=1.000000,G=0.000000,B=0.072804,A=1.000000)" 0.008)
  (Development|PrintString (Utilities|String|ToString(Integer) (Variables|Default|GetDynamic_TotalAntsToSpawn)) true true "(R=0.060965,G=1.000000,B=0.000000,A=1.000000)" 0.008)
  (if (> (Utilities|Array|Length (Variables|Default|GetDynamic_TotalInfectedAnts)) (Utilities|Array|Length (Variables|Default|GetDynamic_TotalHealthyAnts)))
    (Development|PrintText "Alert!" true true "(R=0.000000,G=0.660000,B=1.000000,A=1.000000)" 0.008)
    (Utilities|FlowControl|DoOnce false
      (:Completed
        (for _array_element (Variables|Default|GetDynamic_TotalHealthyAnts)
          (Class|IAntInterface|FunctionAlarmedAlert(Message) _array_element))))))

(event EventFunctionGetAnt
  (params (AntInput :type Actor%20Object%20Reference))
  (Utilities|Array|Add (Variables|Default|GetDynamic_TotalHealthyAnts) AntInput)
  (|WhatAntToSpawn))

(event EventFunctionGetInfectedAnt
  (params (AntInput :type Actor%20Object%20Reference))
  (Utilities|Array|RemoveItem (Variables|Default|GetDynamic_TotalHealthyAnts) AntInput)
  (Utilities|Array|Add (Variables|Default|GetDynamic_TotalInfectedAnts) AntInput)
  (Variables|Default|SetDynamic_TotalAntsToSpawn (- (Variables|Default|GetDynamic_TotalAntsToSpawn) 1)))

(event EventFunctionGetFoodSource
  (params (FoodSource :type Actor%20Object%20Reference))
  (Utilities|Array|Add (Variables|Default|GetDynamic_FoodSources) FoodSource))

(event EventFunctionGetFoodSupply
  (params (FoodSupply :type Actor%20Object%20Reference))
  (Utilities|Array|Add (Variables|Default|GetDynamic_FoodSupplies) FoodSupply))

(event EventFunctionGetAntSpawner
  (params (AntSpawner :type Actor%20Object%20Reference))
  (Utilities|Array|Add (Variables|Default|GetDynamic_AntSpawners) AntSpawner))

(event EventFunctionGetSoldier
  (params (SoldierAnt :type Actor%20Object%20Reference))
  (Utilities|Array|Add (Variables|Default|GetDynamic_TotalAnts_Soldier) SoldierAnt))

(event EventFunctionGetTender
  (params (TenderAnt :type Actor%20Object%20Reference))
  (Utilities|Array|Add (Variables|Default|GetDynamic_TotalAnts_Tender) TenderAnt))

(fn ConstructionScript)

(fn FunctionGiveFoodSupply
  (return (.OutItem (Utilities|Array|Random (Variables|Default|GetDynamic_FoodSupplies)))))

(fn FunctionGiveFoodSource
  (return (.OutItem (Utilities|Array|Random (Variables|Default|GetDynamic_FoodSources)))))

(fn FunctionRemoveInfectedAnt
  (params (InfectedAnt :type Actor%20Object%20Reference))
  (bind _returnvalue (Utilities|Array|RemoveItem (Variables|Default|GetDynamic_TotalInfectedAnts) InfectedAnt))
  (if _returnvalue
    (Development|PrintText "An infected ant died!" true true "(R=0.000000,G=0.660000,B=1.000000,A=1.000000)" 0.2)))

(fn FunctionGiveAntSpawner
  (return (.OutItem (Utilities|Array|Random (Variables|Default|GetDynamic_AntSpawners)))))