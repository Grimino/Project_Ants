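; BP_BaseAbility is a base ability actor for visual feedback that animates a sphere dropping toward a target component.
; Event_StartSphereDrop plays a timeline from the start, feeding its track value as alpha into a relative-location lerp on AbilitySphere.
; The lerp starts from the sphere's current location each update, so movement compounds rather than interpolating from a fixed origin.
; A separate function places the whole actor at a given drop location.
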(event Custom|Event_StartSphereDrop
  (bind _newtrack_0 (Timeline|Timeline_SphereDrop PlayFromStart)
    (:Update
      (|ChangeSphereLocation _newtrack_0))))

(event EventBeginPlay)

(event Collision|EventActorBeginOverlap
  (params (OtherActor :type Actor%20Object%20Reference)))

(event EventTick
  (params (DeltaSeconds :type Float%20%28single-precision%29)))

(fn ConstructionScript)

(fn FunctionSetDropLocation
  (params (NewParam :type Vector))
  (Transformation|SetActorLocation NewParam false false))