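; Actor component that gives click feedback on ants by setting a material on the owner's static mesh.
; On BeginPlay it checks that the owner implements I_AntInterface, binds to its click event through that interface and caches its StaticMeshComponent.
; Each click toggles IsClicked, but both states apply the same material to slot 0.
; An unconnected Smoke_Pipe effect spawn on a leg socket never runs.
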(event Custom|OnMouseClicked
  (params (TouchedActor :type Actor%20Object%20Reference) (ButtonPressed :type Key%20Structure :default "None"))
  (bind _output_get (Variables|Default|SetIsClicked (not (Variables|Default|GetIsClicked))))
  (Utilities|IsValid (Variables|Default|GetStaticMeshRef)
    (:Is%20Valid
      (if _output_get
        _
        (else
          _))
      (Rendering|Material|SetMaterial (Variables|Default|GetStaticMeshRef) 0 "/Game/FO_Folder/AssetsMenu/MM_Window/source/Window/aiStandardSurface8SG.aiStandardSurface8SG"))))

(event EventBeginPlay
  (bind _returnvalue (Components|GetOwner))
  (bind _returnvalue_2 (Actor|GetComponentbyClass _returnvalue "/Script/Engine.StaticMeshComponent"))
  (if (Utilities|DoesObjectImplementInterface _returnvalue "/Game/FrameWorks/Interfaces/I_AntInterface.I_AntInterface_C")
    (EventDispatchers|BindEventtoOnClicked _returnvalue (delegate Custom|OnMouseClicked))
    (Utilities|IsValid _returnvalue_2
      (:Is%20Valid
        (Variables|Default|SetStaticMeshRef _returnvalue_2)))))